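; Floating info text actor that shows its owner's name and a list of needs, each with activity and current value.
; Every Tick it billboards by aligning its X axis with the direction from the player camera to the text.
; SetInfoData stores the needs and calls UpdateInfo before caching the owner's name, so the name appears from later updates.
; UpdateInfo rebuilds the line-broken string, appending any additional info.
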(event EventBeginPlay)

(event EventActorBeginOverlap
  (params (OtherActor :type Actor%20Object%20Reference)))

(event EventTick
  (params (DeltaSeconds :type Float%20%28single-precision%29))
  (Transformation|SetActorRotation (Math|Rotator|MakeRotfromX (- (Transformation|GetWorldLocation (Variables|Default|GetText)) (Transformation|GetActorLocation (Game|GetPlayerCameraManager 0))))))

(fn ConstructionScript)

(fn SetInfoData
  (params (Data :type Array%20of%20NPC%20Need%20Structures))
  (Variables|Default|SetListOfNeeds Data)
  (CallFunction|UpdateInfo)
  (Variables|Default|SetOwnerName (Utilities|GetDisplayName (Components|GetOwner))))

(fn UpdateInfo
  (params (Additional%20Info :type String))
  (bind _output_get (LocalVariables|SetNewText (Utilities|String|Append (Variables|Default|GetOwnerName) "<br>")))
  (for _array_element (Variables|Default|GetListOfNeeds)
    (bind _output_get_2 (LocalVariables|SetNewText (Utilities|String|Append _output_get (Utilities|String|Append (Utilities|String|Append (Utilities|String|MakeLiteralString (Utilities|String|EnumtoString (.Activity (Utilities|Struct|BreakNPCNeed _array_element)))) (Utilities|String|ToString(Float) (.CurrentValue (Utilities|Struct|BreakNPCNeed _array_element)))) "<br>")))))
  (LocalVariables|SetNewText (Utilities|String|Append _output_get_2 Additional%20Info))
  (Rendering|Components|TextRender|SetText (Variables|Default|GetText) (LocalVariables|GetNewText)))