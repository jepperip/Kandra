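; SmartTerrainGameMode is a game mode that supplies a world-size value and a one-time logging start for the smart terrain game.
; GetWorldMaxDistance lazily caches the Diameter of the first Ground actor found, searching again only while the cached value is zero.
; StartLogging passes NeedLabels to StartNewSession behind a DoOnce, and BeginPlay, Tick and the construction script are empty.
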(event EventBeginPlay)

(event EventTick
  (params (DeltaSeconds :type Float%20%28single-precision%29)))

(fn ConstructionScript)

(fn GetWorldMaxDistance
  (if (!= (Variables|SmartProperty|GetWorldMaxDistance) 0.0)
    _
    (else
      (bind _outactors (Actor|GetAllActorsOfClass "/Game/Maps/Ground.Ground_C"))
      (bind _asground (Utilities|Casting|CastToGround (Utilities|Array|Get(acopy) _outactors)))
      (Variables|SmartProperty|SetWorldMaxDistance (Variables|/Game/Maps/Ground.Ground_C|GetDiameter _asground))))
  (return (Variables|SmartProperty|GetWorldMaxDistance)))

(fn StartLogging
  (params (NeedLabels :type Array%20of%20Strings))
  (Utilities|FlowControl|DoOnce false
    (:Completed
      (Class|SmartTerrainFunctions|StartNewSession NeedLabels))))