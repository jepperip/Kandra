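; KandraController is a controller Blueprint with keyboard shortcuts for adjusting game speed and rebuilding navigation.
; It caches the global time dilation on BeginPlay, then the Add and Subtract keys step it by one with no clamping in the graph.
; Each step applies the new dilation and broadcasts it through TimeDialationChanged.
; F5 runs the RebuildNavigation console command.
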(event EventBeginPlay
  (Variables|Default|SetCurrentTimeDialation (Class|GameplayStatics|GetGlobalTimeDilation)))

(event EventTick
  (params (DeltaSeconds :type Float%20%28single-precision%29)))

(event Input|KeyboardEvents|Subtract
  (:Pressed
    (Variables|Default|SetCurrentTimedialation (- (Variables|Default|GetCurrentTimedialation) 1.0))
    (Utilities|Time|SetGlobalTimeDilation (Variables|Default|GetCurrentTimedialation))
    (Default|CallTimeDialationChanged (Variables|Default|GetCurrentTimedialation))))

(event Input|KeyboardEvents|Add
  (:Pressed
    (Variables|Default|SetCurrentTimedialation (+ (Variables|Default|GetCurrentTimedialation) 1.0))
    (Utilities|Time|SetGlobalTimeDilation (Variables|Default|GetCurrentTimedialation))
    (Default|CallTimeDialationChanged (Variables|Default|GetCurrentTimedialation))))

(event Input|KeyboardEvents|F5
  (:Pressed
    (Development|ExecuteConsoleCommand "RebuildNavigation")))

(fn ConstructionScript)