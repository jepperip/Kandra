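; TimerUtility is a game clock that counts hours, minutes and seconds on a compressed scale.
; An Update event, separate from the empty Tick, accumulates delta time, calls SecondTick about once a second and prints the time.
; Seconds roll into minutes after passing 10 and minutes into hours at 24, while hours never wrap.
; Getter functions expose the current second, minute and hour.
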(event Custom|Update
  (params (DeltaSeconds :type Float%20%28single-precision%29))
  (Utilities|FlowControl|Sequence
    (:then_0
      (Variables|Default|SetSecondCounter (+ (Variables|Default|GetSecondCounter) DeltaSeconds))
      (if (>= (Variables|Default|GetSecondCounter) 1.0)
        (Variables|Default|SetSeconds (+ (Variables|Default|GetSecondCounter) (Variables|Default|GetSeconds)))
        (Variables|Default|SetSecondCounter 0.0)
        (Default|CallSecondTick)
        (Development|PrintString (Utilities|String|Append (Utilities|String|Append (Utilities|String|Append (Utilities|String|Append (Utilities|String|Append "H: " (Utilities|String|ToString(Integer) (Variables|Default|GetHours))) "M:") (Utilities|String|ToString(Integer) (Variables|Default|GetMinutes))) "S:") (Utilities|String|ToString(Integer) (+ (Math|Float|Floor (Variables|Default|GetSeconds)) 0))))))
    (:then_1
      (if (> (Variables|Default|GetSeconds) 1e+01)
        (Variables|Default|SetMinutes (+ (Variables|Default|GetMinutes) 1))
        (Variables|Default|SetSeconds 0.0)))
    (:then_2
      (if (>= (Variables|Default|GetMinutes) 24)
        (Variables|Default|SetHours (+ (Variables|Default|GetHours) 1))
        (Variables|Default|SetMinutes 0)))))

(event EventTick
  (params (DeltaSeconds :type Float%20%28single-precision%29)))

(fn ConstructionScript)

(fn GetCurrentSecond
  (return (Math|Float|Floor (Variables|Default|GetSeconds))))

(fn GetCurrentHour
  (return (Variables|Default|GetHours)))

(fn GetCurrentMinute
  (return (Variables|Default|GetMinutes)))