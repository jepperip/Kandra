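; SmartNPC is a smart terrain AI character that moves toward actors broadcasting to it.
; On begin play it binds to its SmartTerrainNPCController's second tick dispatcher, recalculating its current need and deciding what to do on each dispatch.
; AddBroadcast collects incoming broadcasts, which EvaluateBroadcasts judges so the AI controller can move the NPC to the winning sender.
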(event Custom|OnSecondTick
  (Class|SmartNPC|CalculateCurrentNeed)
  (CallFunction|DecideWhattoDo))

(event EventBeginPlay
  (bind _returnvalue (AI|GetAIController self))
  (bind _assmart_terrain_npccontroller (Utilities|Casting|CastToSmartTerrainNPCController _returnvalue))
  (bind _output_get (Variables|Default|SetSmartController _assmart_terrain_npccontroller))
  (EventDispatchers|BindEventtoSecondTickDispatcher _output_get (delegate Custom|OnSecondTick)))

(event EventActorBeginOverlap
  (params (OtherActor :type Actor%20Object%20Reference)))

(event EventTick
  (params (DeltaSeconds :type Float%20%28single-precision%29)))

(fn ConstructionScript)

(fn DecideWhattoDo
  (bind _mybroadcasts (Variables|Default|GetmyBroadcasts))
  (if (> (Utilities|Array|Length _mybroadcasts) 0)
    (bind (_winner _returnvalue) (Class|SmartNPC|EvaluateBroadcasts _mybroadcasts))
    (Development|PrintString (Utilities|String|ToString(Float) _returnvalue))
    (bind _returnvalue_2 (AI|GetAIController self))
    (AI|Navigation|MovetoActor _returnvalue_2 (.Sender (Utilities|Struct|BreakSmartBroadcast _winner)) -1.0 true true false)))

(fn AddBroadcast
  (params (b :type Smart%20Broadcast%20Structure))
  (Utilities|Array|Add (Variables|Default|GetmyBroadcasts) b)
  (return true))